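; BP_HealthbasedSpectatorPawn is a pawn that exercises a health component, CPPHealth, through debug keyboard input.
; The Add and Subtract keys call RecoverHealth and TakeDamage on the component, each with a random amount.
; Tick prints the component's current health every frame.
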(event EventTick
  (params (DeltaSeconds :type Float%20%28single-precision%29))
  (Development|PrintString (Utilities|String|ToString(Float) (Class|CPPHealthComponent|GetHealth (Variables|Default|GetCPP_Health)))))

(event Input|KeyboardEvents|Add
  (params (Key :type Key%20Structure :default "None"))
  (:Pressed
    (Class|CPPHealthComponent|RecoverHealth (Variables|Default|GetCPP_Health) (Math|Random|RandomFloatinRange 0.0 2e+01))))

(event Input|KeyboardEvents|Subtract
  (params (Key :type Key%20Structure :default "None"))
  (:Pressed
    (Class|CPPHealthComponent|TakeDamage (Variables|Default|GetCPP_Health) (Math|Random|RandomFloatinRange 0.0 2e+01))))

(fn ConstructionScript)